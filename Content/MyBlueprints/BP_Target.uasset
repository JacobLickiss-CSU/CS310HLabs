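; BP_Target is a shootable target that the player destroys with first-person projectiles to progress toward a goal.
; Each projectile hit destroys the projectile, lowers the clamped Health and updates the HealthText display.
; At zero health, Broken increments TargetsHit on the player character, calls its CheckGoal and destroys the target.
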(event Custom|Broken
  (bind _asbp_first_person_character (Utilities|Casting|CastToBP_FirstPersonCharacter (Game|GetPlayerCharacter 0)))
  (Variables|/Game/FirstPerson/Blueprints/BP_FirstPersonCharacter.BP_FirstPersonCharacter_C|SetTargetsHit _asbp_first_person_character (+ (Variables|/Game/FirstPerson/Blueprints/BP_FirstPersonCharacter.BP_FirstPersonCharacter_C|GetTargetsHit _asbp_first_person_character) 1))
  (Default|CheckGoal _asbp_first_person_character)
  (Actor|DestroyActor))

(event Collision|EventHit
  (params (MyComp :type Primitive%20Component%20Object%20Reference) (Other :type Actor%20Object%20Reference) (OtherComp :type Primitive%20Component%20Object%20Reference) (bSelfMoved :type Boolean) (HitLocation :type Vector :default "0, 0, 0") (HitNormal :type Vector :default "0, 0, 0") (NormalImpulse :type Vector :default "0, 0, 0") (Hit :type Hit%20Result%20Structure%20%28by%20ref%29))
  (bind _asbp_first_person_projectile (Utilities|Casting|CastToBP_FirstPersonProjectile Other))
  (Actor|DestroyActor _asbp_first_person_projectile)
  (bind _output_get (Variables|Default|Sethealth (Math|Integer|Clamp(Integer) (- (Variables|Default|Gethealth) 20) 0 100)))
  (Rendering|Components|TextRender|SetText (Variables|Default|GetHealthText) (Utilities|Text|ToText(Integer) _output_get))
  (if (<= _output_get 0)
    (CallFunction|Broken)))

(fn ConstructionScript)